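; Selection indicator component for RTS units that shows or hides a decal on its owning actor.
; On BeginPlay it adds a rotated DecalComponent to the owner, applies the selection indicator material and hides it.
; It sizes the decal from IndicatorScale divided by the decal's size, then positions it at IndicatorOFFSET.
; ShowSelectionDecal and HideSelectionDecal toggle both visibility and hidden-in-game state.
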(event `self.ReceiveBeginPlay`
  (bind _indicatorscale (`self.IndicatorScale`))
  (bind (_decalsize_x _decalsize_y _decalsize_z) (`KismetMathLibrary.BreakVector` (`DecalComponent.DecalSize` (`self.DecalComponentRef`))))
  (bind _returnvalue (`|AddComponentByClass` (`self.GetOwner`) "/Script/Engine.DecalComponent" false (`KismetMathLibrary.MakeTransform` (0.0 0.0 0.0) (struct :`Pitch` -90.0))))
  (set `self.DecalComponentRef` _returnvalue)
  (`DecalComponent.SetDecalMaterial` (`self.DecalComponentRef`) "/Game/MyRTS/Core/Building/MI_SelectionIndicator_Inst.MI_SelectionIndicator_Inst")
  (`self.HideSelectionDecal`)
  (`SceneComponent.SetRelativeScale3D` (`self.DecalComponentRef`) (`KismetMathLibrary.MakeVector` 128.0 (/ _indicatorscale _decalsize_y) (/ _indicatorscale _decalsize_z)))
  (`SceneComponent.K2_SetRelativeLocation` (`self.DecalComponentRef`) (`self.IndicatorOFFSET`) false false))

(event `ShowSelectionDecal`
  (bind _decalcomponentref (`self.DecalComponentRef`))
  (`SceneComponent.SetVisibility` _decalcomponentref true false)
  (`SceneComponent.SetHiddenInGame` _decalcomponentref false false))

(event `HideSelectionDecal`
  (bind _decalcomponentref (`self.DecalComponentRef`))
  (`SceneComponent.SetVisibility` _decalcomponentref false false)
  (`SceneComponent.SetHiddenInGame` _decalcomponentref true false))