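; BP_resourceComponent is a component for an RTS resource that can be mined a limited number of times.
; GiveResources decrements the remaining mine count, fires the OnResourceGathered dispatcher and returns the resource type and amount.
; It also fires OnResourceExhausted once CanThisResourceBeMIned reports no mines left.
; GiveResources does not check availability before decrementing, and BeginPlay is empty.
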(event `self.ReceiveBeginPlay`)

(fn `CanThisResourceBeMIned`
  (returns (ReturnValue :type Boolean))
  (return (> (`self.TimeCanMine`) 0)))

(fn `GiveResources`
  (returns (TypeOfResource :type "/Game/MyRTS/Core/Resourse/E_ResourceType Enum") (NumberOfResources :type Integer))
  (set `self.TimeCanMine` (- (`self.TimeCanMine`) 1))
  (`self.OnResourceGathered`)
  (`|ExecutionSequence`
    (:`then_0`
      (if (not (`self.CanThisResourceBeMIned`))
        (`self.OnResourceExhausted`)))
    (:`then_1`
      (return (`self.TypeOfResource`) (`self.NumberOfResources`)))))