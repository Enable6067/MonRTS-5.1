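; RTS game mode that tracks main camps and handles the lose condition.
; On BeginPlay it caches every BP_MainCamp and binds to each building component's destroyed event.
; A destroyed Friendly camp puts the WBP_LoseTheGame widget on screen.
; GetPlayerMainCamp searches for the "Player" tag, but indexes the camp array with the tag's position within that actor's Tags, not the camp's index.
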(event `self.ReceiveBeginPlay`
  (bind _outactors (`GameplayStatics.GetAllActorsOfClass` "/Game/MyRTS/Buildings/BP_MainCamp.BP_MainCamp_C"))
  (bind _output_get (set `self.MainCamp` _outactors))
  (for _array_element _output_get
    (add `/Game/MyRTS/Core/Building/BP_BuildingComponent.OnBuildingDestroyed` (`self.GetComponentByClass` _array_element "/Game/MyRTS/Core/Building/BP_BuildingComponent.BP_BuildingComponent_C") (delegate `OnMainCampDestroyed`))))

(event `OnMainCampDestroyed`
  (params (TeamAttitude :type "ETeamAttitude Enum" :default "Friendly"))
  (if (`|EnumEquality` TeamAttitude "Friendly")
    (`self.LoseTheGame`)))

(event `LoseTheGame`
  (bind _returnvalue (`|CreateWidget` "/Game/MyRTS/UI/Screens/WBP_LoseTheGame.WBP_LoseTheGame_C"))
  (`UserWidget.AddToViewport` _returnvalue 0))

(fn `GetPlayerMainCamp`
  (returns (PlayerMainCamp :type "Actor Object Reference"))
  (for _array_element (`self.MainCamp`)
    (bind _returnvalue (`KismetArrayLibrary.Array_Find` (`Actor.Tags` _array_element) "Player"))
    (if (>= _returnvalue 0)
      (set `self.FoundIndex` _returnvalue)))
  (return (`|GetArrayItem` (`self.MainCamp`) (`self.FoundIndex`))))

(fn `UserConstructionScript`)