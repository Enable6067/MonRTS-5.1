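; BP_ResourceGaratherIndicator is a short-lived RTS actor that acts as a visual indicator for resource gathering, showing a rising mesh.
; The construction script applies the MeshToUse variable to the ResourceMESH component.
; On BeginPlay, a sped-up timeline drives the mesh's relative Z up to UpwardDistance using its alpha curve, then destroys the actor when finished.
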(event `self.ReceiveBeginPlay`
  (`TimelineComponent.SetPlayRate` (`self.UpwardsAnimation`) 1.7)
  (bind (_direction _valuealpha) (`Timeline|UpwardsAnimation`)
    (:`Update`
      (`SceneComponent.K2_SetRelativeLocation` (`self.ResourceMESH`) (`KismetMathLibrary.MakeVector` 0.0 0.0 (* _valuealpha (`self.UpwardDistance`))) false false))
    (:`Finished`
      (`self.K2_DestroyActor`))))

(fn `UserConstructionScript`
  (`StaticMeshComponent.SetStaticMesh` (`self.ResourceMESH`) (`self.MeshToUse`)))