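; Actor component that gives an RTS building health, an on-building health bar and a destruction notification.
; On BeginPlay it adds a health bar widget component to its owner at a configurable offset and size, then binds to the owner's damage event.
; Damage lowers Health, clamped at zero, and refreshes the bar's fill ratio.
; At zero it broadcasts OnBuildingDestroyed with its TeamAttitude, leaving actor removal to other code.
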(event `self.ReceiveBeginPlay`
  (`|ExecutionSequence`
    (:`then_0`
      (bind _returnvalue (`|AddComponentByClass` (`self.GetOwner`) "/Game/MyRTS/Core/Unit/BP_HealthBarWidgetComponent.BP_HealthBarWidgetComponent_C" false (`KismetMathLibrary.MakeTransform` (`self.HealthBarRelativeLocation`))))
      (`WidgetComponent.SetDrawSize` _returnvalue (`self.HealthBarDrawSized`))
      (`self.UndateHealthBar`))
    (:`then_1`
      (add `Actor.OnTakeAnyDamage` (`self.GetOwner`) (`|CreateDelegate` :!event `OnOwnerTakeAnyDamage`)))))

(event `OnOwnerTakeAnyDamage`
  (params (DamagedActor :type "Actor Object Reference") (Damage :type "Float (single-precision)") (DamageType :type "DamageType Object Reference") (InstigatedBy :type "Controller Object Reference") (DamageCauser :type "Actor Object Reference"))
  (set `self.Health` (`KismetMathLibrary.FMax` (- (`self.Health`) Damage)))
  (`self.UndateHealthBar`)
  (if (<= (`self.Health`) 0.0)
    (`self.OnBuildingDestroyed` (`self.TeamAttitude`))))

(fn `UndateHealthBar`
  (bind _returnvalue (`Actor.GetComponentByClass` (`self.GetOwner`) "/Game/MyRTS/Core/Unit/BP_HealthBarWidgetComponent.BP_HealthBarWidgetComponent_C"))
  (`/Engine/EditorBlueprintResources/StandardMacros.IsValid` _returnvalue
    (:`Is Valid`
      (`/Game/MyRTS/Core/Unit/BP_HealthBarWidgetComponent.UpdateHealthBar` _returnvalue (/ (`self.Health`) (`self.HealthMax`))))
    (:`Is Not Valid`
      (`KismetSystemLibrary.PrintString` "ActorNOComponent"))))