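; BP_Building is a clickable RTS building actor that supports selection and removal on destruction.
; A click fires BuildingClickEvent, which adds the building to PlayerControllerRTS's selected-actor list and shows its SelectionDecal.
; DeselectTHIS hides the decal again.
; The actor destroys itself when its BP_BuildingComponent reports OnBuildingDestroyed.
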(event `self.ReceiveActorOnClicked`
  (params (ButtonPressed :type "Key Structure"))
  (`self.BuildingClickEvent`))

(event `BuildingClickEvent`
  (bind _selectiondecal (`self.SelectionDecal`))
  (`|ExecutionSequence`
    (:`then_0`
      (bind _asplayer_controller_rts (cast `/Game/MyRTS/Core/Player/PlayerControllerRTS` (`GameplayStatics.GetPlayerController` 0)))
      (`/Game/MyRTS/Core/Player/PlayerControllerRTS.ADDActorSelected to list` _asplayer_controller_rts self))
    (:`then_1`
      (`SceneComponent.SetHiddenInGame` _selectiondecal false false)
      (`SceneComponent.SetVisibility` _selectiondecal true false))))

(event `/Game/MyRTS/Core/Building/BP_SelectionEvents.DeselectTHIS`
  (bind _selectiondecal (`self.SelectionDecal`))
  (`SceneComponent.SetHiddenInGame` _selectiondecal true false)
  (`SceneComponent.SetVisibility` _selectiondecal false false))

(event `self.BP_BuildingComponent.OnBuildingDestroyed`
  (`self.K2_DestroyActor`))

(fn `UserConstructionScript`)