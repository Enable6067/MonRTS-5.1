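; RTS worker unit that moves on command, gathers and deposits resources, attacks actors and shows a selection decal.
; Each order runs AI MoveTo and sets the BP_UnitComponent state, whose change event plays the looping animation.
; Gathering waits out the resource's time, delivers the load to the main camp for the player controller, then repeats.
; Attacks apply damage on a looping timer, re-approaching when the target exceeds the distance recorded on arrival.
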(event `self.BP_UnitComponent.OnEnterNewState`
  (params (NewState :type "/Game/MyRTS/Core/Unit/E_UnitStates Enum" :default "NewEnumerator0"))
  ;[1 1 1] Анимашки персонажа
  (`SkeletalMeshComponent.PlayAnimation` (`self.Mesh`) (select `/Game/MyRTS/Core/Unit/E_UnitStates` NewState :`NewEnumerator1` "/Game/RTSAssets/Characters/DwarfGrunt/Anims/Idle_1_new.Idle_1_new" :`NewEnumerator2` "/Game/RTSAssets/Characters/DwarfGrunt/Anims/WalkFwd2.WalkFwd2" :`NewEnumerator3` "/Game/RTSAssets/Characters/DwarfGrunt/Anims/AnimMontageAttack_1_new.AnimMontageAttack_1_new" :`NewEnumerator4` "/Game/RTSAssets/Characters/DwarfGrunt/Anims/AnimMontageAttack_1_new.AnimMontageAttack_1_new" :!type "AnimationAsset Object Reference") true))

(event `self.MoveToThisLocation`
  (params (GoalLocation :type "Vector Structure"))
  ;[1 1 1] Move location
  (`/Game/MyRTS/Core/Unit/BP_UnitComponent.HandleUnitState` (`self.BP_UnitComponent`) "NewEnumerator2")
  (bind _movementresult (`|AIMoveTo` self GoalLocation null 50.0)
    (:`OnSuccess`
      _)
    (:`OnFail`
      (switch `EPathFollowingResult` _movementresult
        (:`Blocked`
          _)
        (:`OffPath`
          _)
        (:`Invalid`
          _))))
  (`/Game/MyRTS/Core/Unit/BP_UnitComponent.HandleUnitState` (`self.BP_UnitComponent`) "NewEnumerator1"))

(event `self.GathedTHisResource`
  (params (ResourceREF :type "Actor Object Reference"))
  (bind _returnvalue (`self.GetComponentByClass` ResourceREF "/Game/MyRTS/Core/Resourse/BP_resourceComponent.BP_resourceComponent_C"))
  (bind (_returnvalue_roll _returnvalue_pitch _returnvalue_yaw) (`KismetMathLibrary.BreakRotator` (`KismetMathLibrary.FindLookAtRotation` (`self.K2_GetActorLocation`) (`self.K2_GetActorLocation` ResourceREF))))
  ;[1 1 1] Идти к ресурсам и смотреть на них
  (`/Game/MyRTS/Core/Unit/BP_UnitComponent.HandleUnitState` (`self.BP_UnitComponent`) "NewEnumerator2")
  (`|AIMoveTo` self (0.0 0.0 0.0) ResourceREF 200.0
    (:`OnSuccess`
      (`self.K2_SetActorRotation` (`KismetMathLibrary.MakeRotator` 0.0 0.0 _returnvalue_yaw))
      ;[1 1 1] Сбор ресурсов
      (if (and (`/Game/MyRTS/Core/Resourse/BP_resourceComponent.CanThisResourceBeMIned` _returnvalue) (`|EnumInequality` (`self.ResourceBeingCarring`) (`/Game/MyRTS/Core/Resourse/BP_resourceComponent.TypeOfResource` _returnvalue)))
        (`/Game/MyRTS/Core/Unit/BP_UnitComponent.HandleUnitState` (`self.BP_UnitComponent`) "NewEnumerator3")
        (set `self.AmountOFResource` 0)
        (`KismetSystemLibrary.RetriggerableDelay` (`/Game/MyRTS/Core/Resourse/BP_resourceComponent.TimeToBeGathered` _returnvalue))
        ;[1 1 1] Подбор ресурсов
        (if (`|EnumEquality` (`/Game/MyRTS/Core/Unit/BP_UnitComponent.UnitState` (`self.BP_UnitComponent`)) "NewEnumerator3")
          (bind (_typeofresource _numberofresources) (`/Game/MyRTS/Core/Resourse/BP_resourceComponent.GiveResources` _returnvalue))
          (set `self.ResourceBeingCarring` _typeofresource)
          (set `self.AmountOFResource` _numberofresources)
          (`self.GotoMAINCAMPanddeposite` ResourceREF))
        (elif (and (`|EnumEquality` (`self.ResourceBeingCarring`) (`/Game/MyRTS/Core/Resourse/BP_resourceComponent.TypeOfResource` _returnvalue)) (> (`self.AmountOFResource`) 0))
          (`self.GotoMAINCAMPanddeposite` ResourceREF)
          (else
            (`/Game/MyRTS/Core/Unit/BP_UnitComponent.HandleUnitState` (`self.BP_UnitComponent`) "NewEnumerator1")))))))

(event `self.AttackThisActor`
  (params (ActorToAttack :type "Actor Object Reference"))
  (bind _actor_to_attack (`self.Actor to Attack`))
  (bind _returnvalue (`self.GetComponentByClass` (`self.Actor to Attack`) "/Game/MyRTS/Core/Building/BP_BuildingComponent.BP_BuildingComponent_C"))
  (bind (_returnvalue_roll _returnvalue_pitch _returnvalue_yaw) (`KismetMathLibrary.BreakRotator` (`KismetMathLibrary.FindLookAtRotation` (`self.K2_GetActorLocation`) (`self.K2_GetActorLocation` (`self.Actor to Attack`)))))
  ;[1 1 1] Атака
  (set `self.Actor to Attack` ActorToAttack)
  (`/Game/MyRTS/Core/Unit/BP_UnitComponent.HandleUnitState` (`self.BP_UnitComponent`) "NewEnumerator2")
  (`/Engine/EditorBlueprintResources/StandardMacros.IsValid` _returnvalue
    (:`Is Valid`
      (`|AIMoveTo` self (`SceneComponent.K2_GetComponentLocation` (`/Game/MyRTS/Core/Building/BP_BuildingComponent.GetSutableLocation` _returnvalue)) null 50.0 true
        (:`OnSuccess`
          _)))
    (:`Is Not Valid`
      (`|AIMoveTo` self (0.0 0.0 0.0) (`self.Actor to Attack`) 200.0 true
        (:`OnSuccess`
          _))))
  (`/Engine/EditorBlueprintResources/StandardMacros.IsValid` _actor_to_attack
    (:`Is Valid`
      (set `self.RangeToActorToAttack` (`KismetMathLibrary.Vector_Distance` (`self.K2_GetActorLocation` _actor_to_attack) (`self.K2_GetActorLocation`)))
      (`self.K2_SetActorRotation` (`KismetMathLibrary.MakeRotator` 0.0 0.0 _returnvalue_yaw))
      (`/Game/MyRTS/Core/Unit/BP_UnitComponent.HandleUnitState` (`self.BP_UnitComponent`) "NewEnumerator4")
      (bind _returnvalue_2 (`KismetSystemLibrary.K2_SetTimerDelegate` (`|CreateDelegate` :!event `Attack`) 1.0 true))
      (set `self.AttackTimer` _returnvalue_2))
    (:`Is Not Valid`
      (`self.StopAttack`))))

(event `StopAttack`
  ;[1 1 1] Атака
  (`/Game/MyRTS/Core/Unit/BP_UnitComponent.HandleUnitState` (`self.BP_UnitComponent`) "NewEnumerator1")
  (`KismetSystemLibrary.K2_ClearAndInvalidateTimerHandle` (`self.AttackTimer`)))

(event `Attack`
  (bind _actor_to_attack (`self.Actor to Attack`))
  ;[1 1 1] Атака
  (`self.Actor to Attack`
    (:`then`
      (if (<= (`KismetMathLibrary.Vector_Distance` (`self.K2_GetActorLocation` (`self.Actor to Attack`)) (`self.K2_GetActorLocation`)) (`self.RangeToActorToAttack`))
        (`GameplayStatics.ApplyDamage` (`self.Actor to Attack`) (`/Game/MyRTS/Core/Unit/BP_UnitComponent.DamageToapply` (`self.BP_UnitComponent`)) null null "/Engine/EngineDamageTypes/DmgTypeBP_Environmental.DmgTypeBP_Environmental_C")
        (else
          (`KismetSystemLibrary.K2_ClearAndInvalidateTimerHandle` (`self.AttackTimer`))
          (if (`|EnumEquality` (`/Game/MyRTS/Core/Unit/BP_UnitComponent.UnitState` (`self.BP_UnitComponent`)) "NewEnumerator4")
            (`/Engine/EditorBlueprintResources/StandardMacros.IsValid` _actor_to_attack
              (:`Is Valid`
                (`self.AttackThisActor` _actor_to_attack)))))))
    (:`else`
      (`self.StopAttack`))))

(event `GotoMAINCAMPanddeposite`
  (params (resourceREF :type "Actor Object Reference"))
  (`/Game/MyRTS/Core/Unit/BP_UnitComponent.HandleUnitState` (`self.BP_UnitComponent`) "NewEnumerator2")
  (bind _asgm_rts (cast `/Game/MyRTS/Core/Framework/GM_RTS` (`GameplayStatics.GetGameMode`)))
  (bind _sitabl_elocationref (`/Game/MyRTS/Core/Building/BP_BuildingComponent.GetSutableLocation` (`self.GetComponentByClass` (`/Game/MyRTS/Core/Framework/GM_RTS.GetPlayerMainCamp` _asgm_rts) "/Game/MyRTS/Core/Building/BP_BuildingComponent.BP_BuildingComponent_C")))
  (`/Engine/EditorBlueprintResources/StandardMacros.IsValid` _sitabl_elocationref
    (:`Is Valid`
      (`|AIMoveTo` self (`SceneComponent.K2_GetComponentLocation` _sitabl_elocationref) null 20.0 true
        (:`OnSuccess`
          (`/Game/MyRTS/Core/Unit/BP_UnitComponent.HandleUnitState` (`self.BP_UnitComponent`) "NewEnumerator1")
          (bind _asplayer_controller_rts (cast `/Game/MyRTS/Core/Player/PlayerControllerRTS` (`GameplayStatics.GetPlayerController` 0)))
          (`/Game/MyRTS/Core/Player/PlayerControllerRTS.RecieveResources` _asplayer_controller_rts (`self.ResourceBeingCarring`) (`self.AmountOFResource`))
          (set `self.ResourceBeingCarring` "NewEnumerator0")
          (set `self.AmountOFResource` 0)
          (`/Engine/EditorBlueprintResources/StandardMacros.IsValid` resourceREF
            (:`Is Valid`
              (`self.RepeatMiningAction` resourceREF))))))
    (:`Is Not Valid`
      (`/Game/MyRTS/Core/Unit/BP_UnitComponent.HandleUnitState` (`self.BP_UnitComponent`) "NewEnumerator1"))))

(event `RepeatMiningAction`
  (params (Target :type "Actor Object Reference"))
  (if (`/Game/MyRTS/Core/Resourse/BP_resourceComponent.CanThisResourceBeMIned` (`self.GetComponentByClass` Target "/Game/MyRTS/Core/Resourse/BP_resourceComponent.BP_resourceComponent_C"))
    (`self.GathedTHisResource` Target)))

(event `/Game/MyRTS/Core/Building/BP_SelectionEvents.SelectTHIS`
  (`/Game/MyRTS/Core/Unit/BP_SelectionComponent.ShowSelectionDecal` (`self.BP_SelectionComponent`)))

(event `self.InteractWithBuildoing`
  (params (BuildingREF :type "Actor Object Reference"))
  (bind _returnvalue (`self.GetComponentByClass` BuildingREF "/Game/MyRTS/Core/Building/BP_BuildingComponent.BP_BuildingComponent_C"))
  (`/Engine/EditorBlueprintResources/StandardMacros.IsValid` _returnvalue
    (:`Is Valid`
      (if (> (`self.AmountOFResource`) 0)
        (if (`|EnumEquality` (`/Game/MyRTS/Core/Building/BP_BuildingComponent.TypeOfBuilding` _returnvalue) "NewEnumerator1")
          (`self.GotoMAINCAMPanddeposite` null))))))

(event `/Game/MyRTS/Core/Building/BP_SelectionEvents.DeselectTHIS`
  (`/Game/MyRTS/Core/Unit/BP_SelectionComponent.HideSelectionDecal` (`self.BP_SelectionComponent`)))

(fn `GetTeamAttitude`
  (returns (TeamAttitude :type "ETeamAttitude Enum"))
  (return (`/Game/MyRTS/Core/Unit/BP_UnitComponent.TeamAttitude` (`self.BP_UnitComponent`))))

(fn `UserConstructionScript`)