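; BP_EnemySpawner is an actor that periodically spawns waves of enemy BP_WorkerTribe2 units around itself.
; On BeginPlay it starts a looping timer on SecondToSpawnEnemies, with some variance on the first delay.
; Each wave picks a small random count and spawns that many units at random navigable points within its Sphere radius, raised slightly and always spawned regardless of collision.
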(event `self.ReceiveBeginPlay`
  (bind _returnvalue (`KismetSystemLibrary.K2_SetTimerDelegate` (delegate `SpawnWave`) (`self.SecondToSpawnEnemies`) true 0.0 2.0))
  (set `self.SpawnerTimer` _returnvalue))

(event `SpawnWave`
  (`self.SpawnEnemy` (`KismetMathLibrary.RandomIntegerInRange` 1 5)))

(event `SpawnEnemy`
  (params (EnemysToSpawn :type Integer :default 1))
  (for _ (range 1 (+ EnemysToSpawn 1))
    (bind _randomlocation (`NavigationSystemV1.K2_GetRandomLocationInNavigableRadius` (`self.K2_GetActorLocation`) (`SphereComponent.GetScaledSphereRadius` (`self.Sphere`)) null null))
    (`|SpawnActorFromClass` "/Game/MyRTS/Units/Tribe2/BP_WorkerTribe2.BP_WorkerTribe2_C" (`KismetMathLibrary.MakeTransform` (+ _randomlocation (0.0 0.0 100.0))) "AlwaysSpawn" "OverrideRootScale" null null)))

(fn `UserConstructionScript`)