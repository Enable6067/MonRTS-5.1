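; BP_SelectionUnit is the RTS marquee selection actor that selects friendly units inside a box dragged with the mouse.
; While resizing, Tick stretches a collision box from the actor's location to the cursor hit point and updates the HUD marquee widget.
; Overlaps message the player controller to select friendly selectable actors, or deselect those leaving mid-drag.
; Start and End functions toggle resizing, box collision and the HUD marquee.
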(event `self.ReceiveTick`
  (params (DeltaSeconds :type "Float (single-precision)"))
  (bind (_returnvalue_x _returnvalue_y) (`KismetMathLibrary.BreakVector` (/ (`KismetMathLibrary.Vector_GetAbs` (- (`self.K2_GetActorLocation`) (`self.EndMouseLocation`))) 2.0)))
  ;[1 1 1] Выделение юнитов
  (if (`self.ShouldResizedMarque`)
    (bind _asplayer_controller_rts (cast `/Game/MyRTS/Core/Player/PlayerControllerRTS` (`GameplayStatics.GetPlayerController` 0)))
    (set `self.EndMouseLocation` (`.Location` (`GameplayStatics.BreakHitResult` (`PlayerController.GetHitResultUnderCursorByChannel` _asplayer_controller_rts "TraceTypeQuery1" true))))
    (`SceneComponent.K2_SetWorldLocation` (`self.BoxCol`) (`KismetMathLibrary.VLerp` (`self.K2_GetActorLocation`) (`self.EndMouseLocation`) 0.5) false false)
    (`BoxComponent.SetBoxExtent` (`self.BoxCol`) (`KismetMathLibrary.MakeVector` _returnvalue_x _returnvalue_y 300.0) true)
    (bind _asbp_hud (cast `/Game/MyRTS/Core/Player/BP_HUD` (`PlayerController.GetHUD` (`GameplayStatics.GetPlayerController` 0))))
    (`/Game/MyRTS/Core/Player/WBP_HUD.UpdateMarquee` (`/Game/MyRTS/Core/Player/BP_HUD.HUDWidgetREF` _asbp_hud))))

(event `self.BoxCol.OnComponentBeginOverlap`
  (params (OverlappedComponent :type "PrimitiveComponent Object Reference") (OtherActor :type "Actor Object Reference") (OtherComp :type "PrimitiveComponent Object Reference") (OtherBodyIndex :type Integer) (bFromSweep :type Boolean) (SweepResult :type "HitResult Structure (by ref)"))
  (if (and (`KismetSystemLibrary.DoesImplementInterface` OtherActor "/Game/MyRTS/Core/Building/BP_SelectionEvents.BP_SelectionEvents_C") (`|EnumEquality` (`/Game/MyRTS/Core/Unit/BP_UnitComponent.TeamAttitude` (`self.GetComponentByClass` OtherActor "/Game/MyRTS/Core/Unit/BP_UnitComponent.BP_UnitComponent_C")) "Friendly"))
    (message `/Game/MyRTS/Core/Building/BP_SelectionEvents.SelectTHISactor` (`GameplayStatics.GetPlayerController` 0) OtherActor)))

(event `self.BoxCol.OnComponentEndOverlap`
  (params (OverlappedComponent :type "PrimitiveComponent Object Reference") (OtherActor :type "Actor Object Reference") (OtherComp :type "PrimitiveComponent Object Reference") (OtherBodyIndex :type Integer))
  (if (and (`self.ShouldResizedMarque`) (`KismetSystemLibrary.DoesImplementInterface` OtherActor "/Game/MyRTS/Core/Building/BP_SelectionEvents.BP_SelectionEvents_C"))
    (message `/Game/MyRTS/Core/Building/BP_SelectionEvents.DeSelectTHISactor` (`GameplayStatics.GetPlayerController` 0) OtherActor)))

(fn `EndResizedMarquee`
  (set `self.ShouldResizedMarque` false)
  (`PrimitiveComponent.SetCollisionEnabled` (`self.BoxCol`) "NoCollision")
  (bind _asbp_hud (cast `/Game/MyRTS/Core/Player/BP_HUD` (`PlayerController.GetHUD` (`GameplayStatics.GetPlayerController` 0))))
  (`/Game/MyRTS/Core/Player/WBP_HUD.StopUpdateMarquee` (`/Game/MyRTS/Core/Player/BP_HUD.HUDWidgetREF` _asbp_hud)))

(fn `StartResizedMarquee`
  (set `self.ShouldResizedMarque` true)
  (`PrimitiveComponent.SetCollisionEnabled` (`self.BoxCol`) "QueryOnly")
  (bind _asbp_hud (cast `/Game/MyRTS/Core/Player/BP_HUD` (`PlayerController.GetHUD` (`GameplayStatics.GetPlayerController` 0))))
  (`/Game/MyRTS/Core/Player/WBP_HUD.StartMarqueeUPDATE` (`/Game/MyRTS/Core/Player/BP_HUD.HUDWidgetREF` _asbp_hud)))

(fn `UserConstructionScript`)